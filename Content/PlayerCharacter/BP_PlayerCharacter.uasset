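; BP_PlayerCharacter is the player character, handling movement, yaw-only mouse look, interaction and death.
; InteractSphere overlaps maintain a list of BP_InteractionInterface actors or components, and Interact or TriggerConvo calls OnInteraction on the first entry.
; StartConverastion can also add entries to that list.
; Custom events switch the mesh to single-node idle or death animations, with death leading to a game-over widget and delayed return to MainMenu.
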(event OnComponentBeginOverlap(InteractSphere)
  (params (OverlappedComponent :type Primitive%20Component%20Object%20Reference) (OtherActor :type Actor%20Object%20Reference) (OtherComp :type Primitive%20Component%20Object%20Reference) (OtherBodyIndex :type Integer) (bFromSweep :type Boolean) (SweepResult :type Hit%20Result%20Structure%20%28by%20ref%29))
  ;[1 1 1] Activate off Actor
  (bind _asbp_interaction_interface (Utilities|Casting|CastToBP_InteractionInterface OtherActor)
    (:then
      (Utilities|Array|AddUnique (Variables|Default|GetInteractableInRange) _asbp_interaction_interface))
    (:CastFailed
      ;[1 1 1] Activate off Component
      (for _array_element (Class|Actor|GetComponentsbyInterface OtherActor "/Game/BluePrints/BP_InteractionInterface.BP_InteractionInterface_C")
        (Utilities|Array|AddUnique (Variables|Default|GetInteractableInRange) (.AsBP%20Interaction%20Interface (Utilities|Casting|CastToBP_InteractionInterface _array_element)))))))

(event OnComponentEndOverlap(InteractSphere)
  (params (OverlappedComponent :type Primitive%20Component%20Object%20Reference) (OtherActor :type Actor%20Object%20Reference) (OtherComp :type Primitive%20Component%20Object%20Reference) (OtherBodyIndex :type Integer))
  (bind _asbp_interaction_interface (Utilities|Casting|CastToBP_InteractionInterface OtherActor)
    (:then
      (Utilities|Array|RemoveItem (Variables|Default|GetInteractableInRange) _asbp_interaction_interface))
    (:CastFailed
      (for _array_element (Class|Actor|GetComponentsbyInterface OtherActor "/Game/BluePrints/BP_InteractionInterface.BP_InteractionInterface_C")
        (Utilities|Array|RemoveItem (Variables|Default|GetInteractableInRange) (.AsBP%20Interaction%20Interface (Utilities|Casting|CastToBP_InteractionInterface _array_element)))))))

(event Custom|Active%20Player%20Animation%20Mode
  (bind _mesh (Variables|Character|GetMesh))
  (Components|Animation|SetAnimationMode _mesh "AnimationSingleNode")
  (Components|Animation|SetAnimation _mesh "/Game/ActorCore_Sample_Motions/Pose_dance_catwalk_Female/Idle_Anim.Idle_Anim")
  (Audio|Components|Audio|Play _mesh false)
  (Development|PrintString "Set Animaton"))

(event Custom|Player%20Animtion%20Dead
  (bind _mesh (Variables|Character|GetMesh))
  (Components|Animation|SetAnimationMode _mesh "AnimationSingleNode")
  (Components|Animation|SetAnimation _mesh "/Game/BluePrints/FemaleWalkCycle/FemaleDeath_4.FemaleDeath_4")
  (Audio|Components|Audio|Play _mesh false)
  (Utilities|FlowControl|Delay 3.0)
  (bind _returnvalue (UserInterface|CreateWidget "/Game/Widgets/W_GameOver.W_GameOver_C"))
  (UserInterface|Viewport|AddtoViewport _returnvalue 0)
  (Utilities|FlowControl|Delay 3.0)
  (Game|OpenLevel(byName) "MainMenu"))

(event Custom|Start%20Converastion
  (params (Comp_Interface :type Actor%20Object%20Reference))
  ;[1 1 1] Activate off Actor
  (bind _asbp_interaction_interface (Utilities|Casting|CastToBP_InteractionInterface Comp_Interface)
    (:then
      (Utilities|Array|AddUnique (Variables|Default|GetInteractableInRange) _asbp_interaction_interface)
      (Development|PrintString "Hello"))
    (:CastFailed
      ;[1 1 1] Activate off Component
      (for _array_element (Class|Actor|GetComponentsbyInterface Comp_Interface "/Game/BluePrints/BP_InteractionInterface.BP_InteractionInterface_C")
        (Utilities|Array|AddUnique (Variables|Default|GetInteractableInRange) (.AsBP%20Interaction%20Interface (Utilities|Casting|CastToBP_InteractionInterface _array_element)))))))

(event Custom|Trigger%20Convo
  (if (> (Utilities|Array|Length (Variables|Default|GetInteractableInRange)) 0)
    (Default|OnInteraction (Utilities|Array|Get(acopy) (Variables|Default|GetInteractableInRange)) self)
    (Development|PrintString "Interacted")))

(event Collision|EventActorBeginOverlap
  (params (OtherActor :type Actor%20Object%20Reference)))

(event EventTick
  (params (DeltaSeconds :type Float%20%28single-precision%29)))

(event EventBeginPlay
  (bind _camera (Variables|Default|GetCamera))
  (Class|Controller|SetInitialLocationandRotation (Game|GetPlayerController 0) (Variables|/Script/Engine.SceneComponent|GetRelativeLocation _camera) (Transformation|GetWorldRotation _camera)))

(event Input|ActionEvents|InputActionInteract
  (params (Key :type Key%20Structure :default "None"))
  (:Pressed
    (if (> (Utilities|Array|Length (Variables|Default|GetInteractableInRange)) 0)
      (Default|OnInteraction (Utilities|Array|Get(acopy) (Variables|Default|GetInteractableInRange)) self)
      (Development|PrintString "Interacted"))))

(event Input|AxisEvents|InputAxisMove_Forward/Backard
  (params (AxisValue :type Float%20%28single-precision%29))
  ;[1 1 1] Movment
  (Pawn|Input|AddMovementInput (Math|Vector|GetForwardVector (Math|Rotator|MakeRotator 0.0 0.0 (.Yaw (Math|Rotator|BreakRotator (Pawn|GetControlRotation :!class /Script/Engine.Pawn))))) AxisValue false))

(event Input|AxisEvents|InputAxisMove_Left/Right
  (params (AxisValue :type Float%20%28single-precision%29))
  ;[1 1 1] Movment
  (Pawn|Input|AddMovementInput (Math|Vector|GetRightVector (Math|Rotator|MakeRotator 0.0 0.0 (.Yaw (Math|Rotator|BreakRotator (Pawn|GetControlRotation :!class /Script/Engine.Pawn))))) AxisValue false))

(event Input|AxisEvents|InputAxisMouse_Turn
  (params (AxisValue :type Float%20%28single-precision%29))
  (Pawn|Input|AddControllerYawInput AxisValue))

(event Input|AxisEvents|InputAxisMouse_UpDown
  (params (AxisValue :type Float%20%28single-precision%29)))

(fn ConstructionScript)