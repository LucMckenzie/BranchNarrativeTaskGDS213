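; Behavior tree task that presents a set of player replies in a dialogue conversation and waits for the choice.
; On execute it binds to the reply-finished event of the blackboard's dialogue widget, sends it the replies and switches the player's view to the C_ConvoCamera_1 actor.
; When a reply is chosen, it unbinds, writes the response to the RepliesOut blackboard key and finishes successfully.
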(event Custom|OnReplyFinished
  (params (ChosenResponse :type Integer))
  (EventDispatchers|UnbindEventfromOnReplyFinished (.AsW%20Dialogue%20Widget (Utilities|Casting|CastToW_DialogueWidget (Class|BTFunctionLibrary|GetBlackboardValueasObject (Variables|Default|GetDialogueWidget)))) (delegate Custom|OnReplyFinished))
  (Class|BTFunctionLibrary|SetBlackboardValueasInt (Variables|Default|GetReplies%20%28Out%29) ChosenResponse)
  (AI|BehaviorTree|FinishExecute true))

(event EventReceiveExecuteAI
  (params (OwnerController :type AI%20Controller%20Object%20Reference) (ControlledPawn :type Pawn%20Object%20Reference))
  (bind _dialoguewidget (Variables|Default|GetDialogueWidget))
  (bind _returnvalue (Class|BTFunctionLibrary|GetBlackboardValueasObject _dialoguewidget))
  (bind _asw_dialogue_widget (Utilities|Casting|CastToW_DialogueWidget _returnvalue))
  (EventDispatchers|AssignOnReplyFinished _asw_dialogue_widget (EventDispatchers|CreateEvent :!event Custom|OnReplyFinished))
  (Default|Reply _asw_dialogue_widget (Variables|Default|GetReplies))
  (bind _returnvalue_2 (Actor|GetActorOfClass "/Game/BluePrints/C_ConvoCamera_1.C_ConvoCamera_1_C"))
  (Game|Player|SetViewTargetwithBlend (Game|GetPlayerController 0) _returnvalue_2 0.0 "VTBlend_Linear" 0.0 false))