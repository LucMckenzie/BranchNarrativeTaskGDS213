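; Behavior tree task that closes a dialogue and triggers the "really death" outcome.
; It exits the dialogue widget stored in the blackboard and returns the camera's view target to the player character.
; It then finds the BP_LevelSequence_Test actor, calls ReallyDEATH on it and finishes successfully.
; A 30-second delay before finishing is left unconnected and never runs.
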(event EventReceiveExecuteAI
  (params (OwnerController :type AI%20Controller%20Object%20Reference) (ControlledPawn :type Pawn%20Object%20Reference))
  (Default|Exit (.AsW%20Dialogue%20Widget (Utilities|Casting|CastToW_DialogueWidget (Class|BTFunctionLibrary|GetBlackboardValueasObject (Variables|Default|GetDialogueWidget)))))
  (bind _returnvalue (Actor|GetActorOfClass "/Game/PlayerCharacter/BP_PlayerCharacter.BP_PlayerCharacter_C"))
  (Game|Player|SetViewTargetwithBlend (Game|GetPlayerController 0) _returnvalue 0.0 "VTBlend_Linear" 0.0 false)
  (bind _asbp_level_sequence_test (Utilities|Casting|CastToBP_LevelSequence_TestClass "/Game/BluePrints/LevelSequence/BP_LevelSequence_Test.BP_LevelSequence_Test_C"))
  (bind _returnvalue_2 (Actor|GetActorOfClass _asbp_level_sequence_test))
  (Default|ReallyDEATH _returnvalue_2)
  (AI|BehaviorTree|FinishExecute true))