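; Behavior tree task that has an NPC speak a first-interaction line once.
; It binds to the finished event of the blackboard's dialogue widget, starts the text and switches the player's view to the C_ConvoCamera_2 actor.
; When speech finishes it unbinds, sets a Close flag and finishes successfully, so later executions succeed immediately without speaking.
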(event Custom|OnSpeakFinished
  (EventDispatchers|UnbindEventfromOnSpeakFinished (.AsW%20Dialogue%20Widget (Utilities|Casting|CastToW_DialogueWidget (Class|BTFunctionLibrary|GetBlackboardValueasObject (Variables|Default|GetDialogueWidget)))) (delegate Custom|OnSpeakFinished))
  ;[1 1 1] Creates a one off Interaction
  (Variables|Default|SetClose true)
  (AI|BehaviorTree|FinishExecute true))

(event EventReceiveExecuteAI
  (params (OwnerController :type AI%20Controller%20Object%20Reference) (ControlledPawn :type Pawn%20Object%20Reference))
  (bind _dialoguewidget (Variables|Default|GetDialogueWidget))
  (bind _returnvalue (Class|BTFunctionLibrary|GetBlackboardValueasObject _dialoguewidget))
  (bind _asw_dialogue_widget (Utilities|Casting|CastToW_DialogueWidget _returnvalue))
  (if (Variables|Default|GetClose)
    (AI|BehaviorTree|FinishExecute true)
    (else
      (EventDispatchers|AssignOnSpeakFinished _asw_dialogue_widget (EventDispatchers|CreateEvent :!event Custom|OnSpeakFinished))
      (Default|Speak _asw_dialogue_widget (Variables|Default|GetText))
      (bind _returnvalue_2 (Actor|GetActorOfClass "/Game/BluePrints/C_ConvoCamera_2.C_ConvoCamera_2_C"))
      (Game|Player|SetViewTargetwithBlend (Game|GetPlayerController 0) _returnvalue_2 0.0 "VTBlend_Linear" 0.0 false))))