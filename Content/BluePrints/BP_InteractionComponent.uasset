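; Interaction component that runs a dialogue with the player, driven by a behavior tree.
; BeginPlay spawns a dialogue AI controller solely as a host for the tree.
; OnInteraction shows the dialogue widget, switches to UI-only input, activates the player's animation mode, then runs the tree and passes the widget through the blackboard.
; The widget's exit event restores game input, stops the tree and removes the widget.
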(event Custom|OnExit_Event_0
  (bind _returnvalue (Game|GetPlayerController 0))
  (bind _dialougewidget (Variables|Default|GetDialougeWidget))
  (bind _returnvalue_2 (Widget|GetOwningPlayer _dialougewidget))
  (Input|SetInputModeGameOnly _returnvalue_2)
  (Variables|/Script/Engine.PlayerController|SetbShowMouseCursor _returnvalue_2 false)
  (Input|SetIgnoreMoveInput _returnvalue true)
  (Input|ResetIgnoreMoveInput _returnvalue)
  (AI|Logic|StopLogic (Variables|/Script/AIModule.AIController|GetBrainComponent (Variables|Default|GetAI_Controller)) "")
  (Widget|RemovefromParent (Variables|Default|GetDialougeWidget)))

(event EventBeginPlay
  ;[1 1 1] Only Needed to Create a Behaviour Tree
  (bind _returnvalue (Game|SpawnActorfromClass "/Game/BluePrints/BP_DialogueAIController.BP_DialogueAIController_C" (Math|Transform|MakeTransform "0, 0, 0" "0, 0, 0" "1,1,1") "Undefined" 0 0))
  (Variables|Default|SetAI_Controller _returnvalue))

(event EventOnInteraction
  (params (PlayerCharacter :type BP%20Player%20Character%20Object%20Reference))
  (bind _returnvalue (Pawn|GetController PlayerCharacter))
  (bind _asplayer_controller (Utilities|Casting|CastToPlayerController _returnvalue))
  (bind _returnvalue_2 (UserInterface|CreateWidget "/Game/BluePrints/W_DialogueWidget.W_DialogueWidget_C" _asplayer_controller))
  (bind _output_get (Variables|Default|SetDialougeWidget _returnvalue_2))
  (EventDispatchers|AssignOnExit _output_get (delegate Custom|OnExit_Event_0))
  (UserInterface|Viewport|AddtoViewport _output_get 0)
  (Input|SetInputModeUIOnly _asplayer_controller _output_get "DoNotLock")
  (Input|SetIgnoreMoveInput (Game|GetPlayerController 0) true)
  (Variables|/Script/Engine.PlayerController|SetbShowMouseCursor _asplayer_controller true)
  (bind _asbp_player_character (Utilities|Casting|CastToBP_PlayerCharacter (Game|GetPlayerCharacter 0)))
  (Default|ActivePlayerAnimationMode _asbp_player_character)
  (AI|RunBehaviorTree (Variables|Default|GetAI_Controller) (Variables|Default|GetDialougeTree))
  (bind _blackboardcomponent (Class|AIController|UseBlackboard (Variables|Default|GetAI_Controller) "/Game/BluePrints/DialougeBlackBoard.DialougeBlackBoard"))
  (AI|Components|Blackboard|SetValueasObject _blackboardcomponent (Utilities|Name|MakeLiteralName "Dialoge_Widget") (Variables|Default|GetDialougeWidget)))